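; Candle test Blueprint that runs a minute-based countdown from BeginPlay, with no visual or gameplay effect yet.
; A looping one-second timer counts Seconds up to 60, then resets it and decrements Minutes, which starts one below MaxMinuteTime.
; When Minutes drops below zero, it prints "Finito" and clears the timer through its stored handle.
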(event Custom|Timer
  ;[0.15 0.15 0.15 0.5] Set Up Timer need to know when to activate
  (if (>= (Variables|Default|GetSeconds) 60)
    (Variables|Default|SetSeconds 0)
    (bind _output_get (Variables|Default|SetMinutes (- (Variables|Default|GetMinutes) 1)))
    (if (< _output_get 0)
      (Development|PrintString "Finito")
      (Utilities|Time|ClearandInvalidateTimerbyHandle (Variables|Default|GetTimerHandlerRef)))
    (else
      (bind _result (Math|Integer|IncrementInt (Variables|Default|GetSeconds))))))

(event EventBeginPlay
  ;[0.15 0.15 0.15 0.5] Set Up Timer need to know when to activate
  (Variables|Default|SetMinutes (- (Variables|Default|GetMaxMinuteTime) 1))
  (bind _returnvalue (Utilities|Time|SetTimerbyEvent (delegate Custom|Timer) 1.0 true))
  (Variables|Default|SetTimerHandlerRef _returnvalue))

(fn ConstructionScript)
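; BP_ThrowableObject is an interactable physics object that a player picks up and releases with alternating Interact calls.
; A MultiGate disables sphere physics and attaches it to the interactor's first-person camera, then re-enables physics and detaches it without applying any impulse.
; While held, it is hidden when the interactor is not locally viewed.
; CanInteract toggles the mesh's custom depth rendering and returns its input.
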(event EventInteract
  (params (InteractionActor :type BP%20First%20Person%20Character%20Object%20Reference))
  (Utilities|FlowControl|MultiGate false false -1 :!label _label
    (:Out%200
      (Physics|SetSimulatePhysics (Variables|Default|GetCollisionSphere) false)
      (Transformation|AttachComponentToComponent (Variables|/Game/Blueprints/CharacterBlueprint/BP_FirstPersonCharacter.BP_FirstPersonCharacter_C|GetFirstPersonCamera InteractionActor) "None" "KeepWorld" "KeepWorld" "KeepWorld" true)
      (if (not (Pawn|IsLocallyViewed InteractionActor))
        (Rendering|SetVisibility (Variables|Default|GetCollisionSphere) false true)))
    (:Out%201
      (Physics|SetSimulatePhysics (Variables|Default|GetCollisionSphere) true)
      (Transformation|DetachFromActor "KeepWorld" "KeepWorld" "KeepWorld")
      (if (Pawn|IsLocallyViewed InteractionActor)
        (goto _label Reset)
        (else
          (Rendering|SetVisibility (Variables|Default|GetCollisionSphere) true true)
          (goto _label Reset))))))

(fn ConstructionScript)

(fn CanInteract
  (params (CanInteract :type Boolean))
  (Rendering|SetRenderCustomDepth (Variables|Default|GetStaticMesh) CanInteract)
  (return CanInteract))
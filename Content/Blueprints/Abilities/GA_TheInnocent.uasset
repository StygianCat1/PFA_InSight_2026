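; GA_TheInnocent is a gameplay ability for BP_WalterCharacter; it has no gameplay effect yet beyond managing its own end.
; On activation it caches the player-controlled Walter and polls on a looping quarter-second timer.
; Each poll ends the ability if either capacity slot holds this class while that slot's check flag is false.
; Ending only prints the ability name and performs an unused character cast.
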(event Custom|StopCapacity
  (Utilities|FlowControl|Sequence
    (:then_0
      (bind _requirementmet (CallFunction|StopCapacity1 (stale Ability|EventActivateAbility _asbp_walter_character) (Variables|/Game/Blueprints/CharacterBlueprint/BP_FirstPersonCharacter.BP_FirstPersonCharacter_C|GetCheckCapacity1 (stale Ability|EventActivateAbility _asbp_walter_character))))
      (if _requirementmet
        (Ability|EndAbility :!label _label)))
    (:then_1
      (bind _requirementmet_2 (CallFunction|StopCapacity2 (stale Ability|EventActivateAbility _asbp_walter_character) (Variables|/Game/Blueprints/CharacterBlueprint/BP_FirstPersonCharacter.BP_FirstPersonCharacter_C|GetCheckCapacity2 (stale Ability|EventActivateAbility _asbp_walter_character))))
      (if _requirementmet_2
        (goto _label)))))

(event Ability|EventActivateAbility
  (bind _asbp_walter_character (Utilities|Casting|CastToBP_WalterCharacter (Pawn|GetControlledPawn (Game|GetPlayerController 0))))
  (Utilities|Time|SetTimerbyEvent (delegate Custom|StopCapacity) 0.25 true))

(event Ability|EventOnEndAbility
  (params (bWasCancelled :type Boolean))
  (Development|PrintString "TheInnocent")
  (Utilities|Casting|CastToBP_WalterCharacter (Pawn|GetControlledPawn (Game|GetPlayerController 0))))

(fn StopCapacity1
  (params (CharacterRef :type BP%20First%20Person%20Character%20Object%20Reference) (Check :type Boolean))
  (if (not Check)
    (bind _gameplayabilty1 (Variables|/Game/Blueprints/CharacterBlueprint/BP_FirstPersonCharacter.BP_FirstPersonCharacter_C|GetGameplayAbilty1 CharacterRef)
      (:then
        (return (== _gameplayabilty1 (Utilities|GetClass self))))
      (:else))))

(fn StopCapacity2
  (params (CharacterRef :type BP%20First%20Person%20Character%20Object%20Reference) (Check :type Boolean))
  (if (not Check)
    (bind _gameplayabilty2 (Variables|/Game/Blueprints/CharacterBlueprint/BP_FirstPersonCharacter.BP_FirstPersonCharacter_C|GetGameplayAbilty2 CharacterRef)
      (:then
        (return (== _gameplayabilty2 (Utilities|GetClass self))))
      (:else))))
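; Gameplay ability The Sage for Victoria: while active, it reveals her normally hidden SeeableThingsWithCapacity actors and runs the insight bar.
; Activation sets the insight per-second rate, then a looping timer ends the ability once the capacity check for its assigned slot turns false.
; Ending re-hides the actors, stops bar progression and raises the clamped insight rate multiplier.
; The character is resolved through player controller 0, and bar updates use multicast events.
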(event Custom|StopCapacity
  (Utilities|FlowControl|Sequence
    (:then_0
      (bind _requirementmet (CallFunction|StopCapacity1 (stale Ability|EventActivateAbility _asbp_victoria_character) (Variables|/Game/Blueprints/CharacterBlueprint/BP_FirstPersonCharacter.BP_FirstPersonCharacter_C|GetCheckCapacity1 (stale Ability|EventActivateAbility _asbp_victoria_character))))
      (if _requirementmet
        (Ability|EndAbility :!label _label)))
    (:then_1
      (bind _requirementmet_2 (CallFunction|StopCapacity2 (stale Ability|EventActivateAbility _asbp_victoria_character) (Variables|/Game/Blueprints/CharacterBlueprint/BP_FirstPersonCharacter.BP_FirstPersonCharacter_C|GetCheckCapacity2 (stale Ability|EventActivateAbility _asbp_victoria_character))))
      (if _requirementmet_2
        (goto _label)))))

(event Ability|EventActivateAbility
  (bind _asbp_victoria_character (Utilities|Casting|CastToBP_VictoriaCharacter (Pawn|GetControlledPawn (Game|GetPlayerController 0))))
  (Variables|/Game/Blueprints/CharacterBlueprint/BP_FirstPersonCharacter.BP_FirstPersonCharacter_C|SetInsightPerSeconds _asbp_victoria_character 2.0)
  (for _array_element (Variables|/Game/Blueprints/CharacterBlueprint/BP_FirstPersonCharacter.BP_FirstPersonCharacter_C|GetSeeableThingsWithCapacity _asbp_victoria_character)
    (Rendering|SetActorHiddenInGame _array_element false))
  (Default|Multicast-InsightBarEvent _asbp_victoria_character)
  (Utilities|Time|SetTimerbyEvent (delegate Custom|StopCapacity) 0.25 true))

(event Ability|EventOnEndAbility
  (params (bWasCancelled :type Boolean))
  (bind _asbp_victoria_character (Utilities|Casting|CastToBP_VictoriaCharacter (Pawn|GetControlledPawn (Game|GetPlayerController 0))))
  (for _array_element (Variables|/Game/Blueprints/CharacterBlueprint/BP_FirstPersonCharacter.BP_FirstPersonCharacter_C|GetSeeableThingsWithCapacity _asbp_victoria_character)
    (Rendering|SetActorHiddenInGame _array_element true))
  (Default|Multicast-InsightBarStopProgression _asbp_victoria_character)
  (Variables|/Game/Blueprints/CharacterBlueprint/BP_FirstPersonCharacter.BP_FirstPersonCharacter_C|SetInsightPerSecondsMultiplier _asbp_victoria_character (Math|Float|Clamp(Float) (+ (Variables|/Game/Blueprints/CharacterBlueprint/BP_FirstPersonCharacter.BP_FirstPersonCharacter_C|GetInsightPerSecondsMultiplier _asbp_victoria_character) (/ (Math|Float|MakeLiteralFloat 1.0) (Math|Float|MakeLiteralFloat 3.0))) 1.0 3.0)))

(fn OnRepStop)

(fn StopCapacity1
  (params (CharacterRef :type BP%20First%20Person%20Character%20Object%20Reference) (Check :type Boolean))
  (if (not Check)
    (bind _gameplayabilty1 (Variables|/Game/Blueprints/CharacterBlueprint/BP_FirstPersonCharacter.BP_FirstPersonCharacter_C|GetGameplayAbilty1 CharacterRef)
      (:then
        (return (== _gameplayabilty1 (Utilities|GetClass self))))
      (:else))))

(fn StopCapacity2
  (params (CharacterRef :type BP%20First%20Person%20Character%20Object%20Reference) (Check :type Boolean))
  (if (not Check)
    (bind _gameplayabilty2 (Variables|/Game/Blueprints/CharacterBlueprint/BP_FirstPersonCharacter.BP_FirstPersonCharacter_C|GetGameplayAbilty2 CharacterRef)
      (:then
        (return (== _gameplayabilty2 (Utilities|GetClass self))))
      (:else))))
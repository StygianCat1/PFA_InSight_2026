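; BP_InsightElementBase is a base Blueprint for a world element whose mesh changes with an insight level.
; It shows the level-zero mesh in the construction script and again on BeginPlay.
; SetChange picks one of four meshes by level, but defers the swap until the actor has not been recently rendered, polling on a short delay loop so the change happens unseen.
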(event EventBeginPlay
  (Components|StaticMesh|SetStaticMesh (Variables|Default|GetCube) (Variables|Default|GetMeshInsight0)))

(event EventSetChange
  (params (InsightLevel :type Integer))
  (if (Class|Actor|WasRecentlyRendered 0.2) :!label _label
    (Utilities|FlowControl|Delay 0.5)
    (goto _label)
    (else
      (switch int InsightLevel
        (:0
          (Components|StaticMesh|SetStaticMesh (Variables|Default|GetCube) (Variables|Default|GetMeshInsight0)))
        (:1
          (Components|StaticMesh|SetStaticMesh (Variables|Default|GetCube) (Variables|Default|GetMeshInsight1)))
        (:2
          (Components|StaticMesh|SetStaticMesh (Variables|Default|GetCube) (Variables|Default|GetMeshInsight2)))
        (:3
          (Components|StaticMesh|SetStaticMesh (Variables|Default|GetCube) (Variables|Default|GetMeshInsight3)))))))

(fn ConstructionScript
  (Components|StaticMesh|SetStaticMesh (Variables|Default|GetCube) (Variables|Default|GetMeshInsight0)))
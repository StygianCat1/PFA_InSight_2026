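; Interactable door Blueprint that swings open and closed around a Scene pivot.
; Interact alternates through a MultiGate between playing and reversing the Move timeline, and the gate resets once the reverse finishes.
; The timeline's DoorTrack scales the yaw of the right or left open rotation, chosen by DoorOpeningSide.
; CanInteract swaps the Cube's material to AliasReference.
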(event EventInteract
  (bind _openrightrot (Variables|Default|GetOpenRightRot))
  (bind _openleftrot (Variables|Default|GetOpenLeftRot))
  (Utilities|FlowControl|MultiGate false false -1 :!label _label
    (:Out%200
      (bind (_direction _doortrack) (Timeline|Move Play)
        (:Update
          (switch Utilities|FlowControl|Switch|SwitchonE_DoorSide (Variables|Default|GetDoorOpeningSide)
            (:NewEnumerator0
              (Transformation|SetRelativeRotation (Variables|Default|GetScene) (Math|Rotator|MakeRotator (.roll _openrightrot) (.pitch _openrightrot) (* _doortrack (.yaw _openrightrot))) false false))
            (:NewEnumerator1
              (Transformation|SetRelativeRotation (Variables|Default|GetScene) (Math|Rotator|MakeRotator (.roll _openleftrot) (.pitch _openleftrot) (* _doortrack (.yaw _openleftrot))) false false))))
        (:Finished
          (switch Utilities|FlowControl|Switch|SwitchonETimelineDirection _direction
            (:Backward
              (goto _label Reset))))))
    (:Out%201
      (Timeline|Move Reverse))))

(event EventCanInteract
  (Rendering|Material|SetMaterial (Variables|Default|GetCube) 0 "/DatasmithContent/Materials/AliasReference.AliasReference"))

(fn ConstructionScript)
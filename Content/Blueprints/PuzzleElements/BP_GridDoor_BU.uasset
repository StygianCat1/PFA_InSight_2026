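; BP_GridDoor_BU is a puzzle grid door that swings open when its OpenGrid event is called.
; On BeginPlay it caches every BP_SymbolCylinder in the level.
; OpenGrid destroys the cylinders whose category matches the door's GridCategory, then passes through a DoOnce to play a timeline that yaws the door toward OpenRotationAngle.
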(event Custom|OpenGrid
  (for _array_element (Variables|Default|GetAllCylinders)
    (if (Utilities|Enum|Equal(Enum) (Variables|/Game/Blueprints/PuzzleElements/BP_SymbolCylinder.BP_SymbolCylinder_C|GetCylinderCategory _array_element) (Variables|Default|GetGridCategory))
      (Actor|DestroyActor _array_element)))
  (Utilities|FlowControl|DoOnce false
    (:Completed
      (bind _turndoor (Timeline|Timeline PlayFromStart)
        (:Update
          (Transformation|SetRelativeRotation (Variables|Default|GetGridDoor) (Math|Rotator|MakeRotator 0.0 0.0 (* _turndoor (Variables|Default|GetOpenRotationAngle))) false false))))))

(event EventBeginPlay
  (bind _outactors (Actor|GetAllActorsOfClass "/Game/Blueprints/PuzzleElements/BP_SymbolCylinder.BP_SymbolCylinder_C"))
  (Variables|Default|SetAllCylinders _outactors))

(fn ConstructionScript)
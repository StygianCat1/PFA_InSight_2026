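; BP_SymbolCylinder is an interactable rotating cylinder that acts as one dial of a code puzzle on its parent BP_GridDoor.
; Interact plays the Turn timeline to rotate the cylinder's yaw by one step.
; When the turn finishes, it advances its numbered slot in the door's position array, wrapping after six, and opens the grid if all positions match the target.
; CanInteract toggles custom depth rendering on the cylinder.
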(event EventBeginPlay
  (Variables|Default|SetCylinderRotation (.yaw (Variables|/Script/Engine.SceneComponent|GetRelativeRotation (Variables|Default|GetCodeCylinder))))
  (bind _asbp_grid_door (Utilities|Casting|CastToBP_GridDoor (Actor|GetParentActor self)))
  (Variables|Default|SetCurrentLockedGrid _asbp_grid_door))

(event EventInteract
  (params (InteractionActor :type BP%20First%20Person%20Character%20Object%20Reference))
  (bind _currentlockedgrid (Variables|Default|GetCurrentLockedGrid))
  (bind _codecylinder (Variables|Default|GetCodeCylinder))
  (bind _cylindernumber (Variables|Default|GetCylinderNumber))
  (bind _returnvalue (- _cylindernumber 1))
  (bind _relativerotation (Variables|/Script/Engine.SceneComponent|GetRelativeRotation _codecylinder))
  (bind _cylinderpositions (Variables|/Game/Blueprints/PuzzleElements/BP_GridDoor.BP_GridDoor_C|GetCylinderPositions _currentlockedgrid))
  (bind _output (Utilities|Array|Get(acopy) _cylinderpositions _returnvalue))
  (bind _returnvalue_2 (+ _output 1))
  (Development|PrintString "Hello")
  (bind _turnangle (Timeline|Turn Play)
    (:Update
      (Transformation|SetRelativeRotation _codecylinder (Math|Rotator|MakeRotator (.roll _relativerotation) (.pitch _relativerotation) (+ (Variables|Default|GetCylinderRotation) (* _turnangle (Variables|Default|GetTurnAngle)))) false false))
    (:Finished
      (Utilities|FlowControl|Sequence
        (:then_0
          (Variables|Default|SetCylinderRotation (+ (Variables|Default|GetCylinderRotation) (* _turnangle (Variables|Default|GetTurnAngle))))
          (if (<= _returnvalue_2 6)
            (Utilities|Array|SetArrayElem _cylinderpositions _returnvalue _returnvalue_2)
            (else
              (Utilities|Array|SetArrayElem _cylinderpositions _returnvalue 1)))
          (if (Utilities|Array|Identical _cylinderpositions (Variables|/Game/Blueprints/PuzzleElements/BP_GridDoor.BP_GridDoor_C|GetTargetPositions _currentlockedgrid))
            (Default|OpenGrid _currentlockedgrid)))
        (:then_1
          (Timeline|Turn SetNewTime))))))

(fn ConstructionScript)

(fn CanInteract
  (params (CanInteract :type Boolean))
  (Rendering|SetRenderCustomDepth (Variables|Default|GetCodeCylinder) CanInteract)
  (return false))
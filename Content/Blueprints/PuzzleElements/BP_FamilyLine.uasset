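; BP_FamilyLine is a puzzle element whose line plane turns blue when solved and lights a candle on the eldritch circle.
; BeginPlay caches the level's BP_EldritchCirrcle actor.
; Solve plays a sound at its location, then, once only, swaps the plane to the blue line material, waits briefly, and activates a candle with a 2D ignition sound if the circle is valid.
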(event Custom|Solve
  (Audio|PlaySoundatLocation "/Engine/VREditor/Sounds/UI/Enter_Simulate.Enter_Simulate" (Transformation|GetActorLocation) "0, 0, 0" 1.0 1.0 0.0 0 0 0 0)
  (Utilities|FlowControl|DoOnce false
    (:Completed
      (Rendering|Material|SetMaterial (Variables|Default|GetPlane) 0 "/Game/Textures/Image/M_UI_Line_Blue.M_UI_Line_Blue")
      (Utilities|FlowControl|Delay 1.0)
      (bind _eldritchcircle (Variables|Default|GetEldritchCircle)
        (:then
          (Default|ActivateCandle _eldritchcircle)
          (Audio|PlaySound2D "/Game/Sound/SFX/Base/Importer/Allumage_Bougie.Allumage_Bougie" 1.0 1.0 0.0 0 0))
        (:else)))))

(event EventBeginPlay
  (bind _returnvalue (Actor|GetActorOfClass "/Game/Blueprints/PuzzleElements/BP_EldritchCirrcle.BP_EldritchCirrcle_C"))
  (Variables|Default|SetEldritchCircle _returnvalue))

(fn ConstructionScript)
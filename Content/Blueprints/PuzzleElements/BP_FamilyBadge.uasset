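; BP_FamilyBadge is a puzzle element that toggles one family's state within a parent BP_FamilyTree puzzle, which it finds through GetParentActor on BeginPlay.
; Interact flip-flops the badge material between blue and grey and writes the matching boolean into the tree's FamilyStates at FamilyIndex minus one.
; After each toggle it compares that array to TargetFamilyStates and calls Solve on a match.
; CanInteract always returns false.
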(event EventBeginPlay
  (bind _asbp_family_tree (Utilities|Casting|CastToBP_FamilyTree (Actor|GetParentActor self)))
  (Variables|Default|SetFamily%20Tree _asbp_family_tree))

(event EventInteract
  (params (InteractionActor :type BP%20First%20Person%20Character%20Object%20Reference))
  (bind _badge (Variables|Default|GetBadge))
  (bind _family_tree (Variables|Default|GetFamily%20Tree))
  (bind _familyindex (Variables|Default|GetFamilyIndex))
  (bind _family_tree_2 (Variables|Default|GetFamily%20Tree))
  (bind _returnvalue (- _familyindex 1))
  (bind _familystates (Variables|/Game/Blueprints/PuzzleElements/BP_FamilyTree.BP_FamilyTree_C|GetFamilyStates _family_tree_2))
  (Utilities|FlowControl|FlipFlop
    (:A
      (Rendering|Material|SetMaterial _badge 0 "/Game/Materials/BasicUnrealMaterial/MI_Blue.MI_Blue")
      (Utilities|Array|SetArrayElem _familystates _returnvalue true))
    (:B
      (Rendering|Material|SetMaterial _badge 0 "/Game/Materials/BasicUnrealMaterial/MI_Grey.MI_Grey")
      (Utilities|Array|SetArrayElem _familystates _returnvalue false)))
  (if (Utilities|Array|Identical (Variables|/Game/Blueprints/PuzzleElements/BP_FamilyTree.BP_FamilyTree_C|GetFamilyStates _family_tree) (Variables|/Game/Blueprints/PuzzleElements/BP_FamilyTree.BP_FamilyTree_C|GetTargetFamilyStates _family_tree))
    (Default|Solve _family_tree)))

(fn ConstructionScript)

(fn CanInteract
  (params (CanInteract :type Boolean))
  (return false))
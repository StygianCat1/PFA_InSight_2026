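; BP_Test is an interactable combination-lock cylinder that expects a BP_GridDoor parent actor, cached on BeginPlay.
; Interact plays a timeline that yaws the cylinder by TurnAngle, then advances its CylinderNumber slot in the door's CylinderPositions, wrapping from 6 to 1.
; When the positions match TargetPositions it calls OpenGrid on the door.
; CanInteract toggles custom depth on the cylinder and always returns false.
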(event EventBeginPlay
  (Variables|Default|SetCylinderRotation (.yaw (Variables|/Script/Engine.SceneComponent|GetRelativeRotation (Variables|Default|GetCylinder))))
  (bind _asbp_grid_door (Utilities|Casting|CastToBP_GridDoor (Actor|GetParentActor self)))
  (Variables|Default|SetCurrent%20Locked%20Grid _asbp_grid_door))

(event EventInteract
  (bind _cylinder (Variables|Default|GetCylinder))
  (bind _current_locked_grid (Variables|Default|GetCurrent%20Locked%20Grid))
  (bind _cylindernumber (Variables|Default|GetCylinderNumber))
  (bind _returnvalue (- _cylindernumber 1))
  (bind _relativerotation (Variables|/Script/Engine.SceneComponent|GetRelativeRotation _cylinder))
  (bind _cylinderpositions (Variables|/Game/Blueprints/PuzzleElements/BP_GridDoor.BP_GridDoor_C|GetCylinderPositions _current_locked_grid))
  (bind _output (Utilities|Array|Get(acopy) _cylinderpositions _returnvalue))
  (bind _returnvalue_2 (+ _output 1))
  (Development|PrintString "Hello")
  (bind _turnangle (Timeline|Timeline Play)
    (:Update
      (Transformation|SetRelativeRotation _cylinder (Math|Rotator|MakeRotator (.roll _relativerotation) (.pitch _relativerotation) (+ (Variables|Default|GetCylinderRotation) (* _turnangle (Variables|Default|GetTurnAngle)))) false false))
    (:Finished
      (Utilities|FlowControl|Sequence
        (:then_0
          (Variables|Default|SetCylinderRotation (+ (Variables|Default|GetCylinderRotation) (* _turnangle (Variables|Default|GetTurnAngle))))
          (if (<= _returnvalue_2 6)
            (Utilities|Array|SetArrayElem _cylinderpositions _returnvalue _returnvalue_2)
            (else
              (Utilities|Array|SetArrayElem _cylinderpositions _returnvalue 1)))
          (if (Utilities|Array|Identical _cylinderpositions (Variables|/Game/Blueprints/PuzzleElements/BP_GridDoor.BP_GridDoor_C|GetTargetPositions _current_locked_grid))
            (Default|OpenGrid _current_locked_grid)))
        (:then_1
          (Timeline|Timeline SetNewTime))))))

(fn ConstructionScript)

(fn CanInteract
  (params (CanInteract :type Boolean))
  (Rendering|SetRenderCustomDepth (Variables|Default|GetCylinder) CanInteract)
  (return false))
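; BP_SymbolCylinder_BU is an interactable puzzle cylinder that turns in steps to help unlock grid doors.
; Interacting plays a Turn timeline that rotates CodeCylinder in yaw by TurnAngle.
; When finished, it advances its CylinderNumber slot, wrapping from six to one, on every BP_GridDoor matching CylinderCategory.
; After the loop, it compares only the last iterated door's positions with its targets and opens it on a match.
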(event EventBeginPlay
  (Variables|Default|SetCylinderRotation (.yaw (Transformation|GetWorldRotation (Variables|Default|GetCodeCylinder))))
  (bind _outactors (Actor|GetAllActorsOfClass "/Game/Blueprints/PuzzleElements/BP_GridDoor.BP_GridDoor_C"))
  (Variables|Default|SetAllLockedGrids _outactors))

(event EventInteract
  (bind _cylindernumber (Variables|Default|GetCylinderNumber))
  (bind _returnvalue (- _cylindernumber 1))
  (bind _turnangle (Timeline|Turn PlayFromStart)
    (:Update
      (Transformation|SetWorldRotation (Variables|Default|GetCodeCylinder) (Math|Rotator|MakeRotator 0.0 0.0 (+ (Variables|Default|GetCylinderRotation) (* _turnangle (Variables|Default|GetTurnAngle)))) false false))
    (:Finished
      (Variables|Default|SetCylinderRotation (+ (Variables|Default|GetCylinderRotation) (* _turnangle (Variables|Default|GetTurnAngle))))
      (for _array_element (Variables|Default|GetAllLockedGrids)
        (if (Utilities|Enum|Equal(Enum) (Variables|/Game/Blueprints/PuzzleElements/BP_GridDoor.BP_GridDoor_C|GetGridCategory _array_element) (Variables|Default|GetCylinderCategory))
          (if (<= (+ (Utilities|Array|Get(acopy) (Variables|/Game/Blueprints/PuzzleElements/BP_GridDoor.BP_GridDoor_C|GetCylinderPositions _array_element) _returnvalue) 1) 6)
            (Utilities|Array|SetArrayElem (Variables|/Game/Blueprints/PuzzleElements/BP_GridDoor.BP_GridDoor_C|GetCylinderPositions _array_element) _returnvalue (+ (Utilities|Array|Get(acopy) (Variables|/Game/Blueprints/PuzzleElements/BP_GridDoor.BP_GridDoor_C|GetCylinderPositions _array_element) _returnvalue) 1))
            (else
              (Utilities|Array|SetArrayElem (Variables|/Game/Blueprints/PuzzleElements/BP_GridDoor.BP_GridDoor_C|GetCylinderPositions _array_element) _returnvalue 1)))))
      (if (Utilities|Array|Identical (Variables|/Game/Blueprints/PuzzleElements/BP_GridDoor.BP_GridDoor_C|GetCylinderPositions _array_element) (Variables|/Game/Blueprints/PuzzleElements/BP_GridDoor.BP_GridDoor_C|GetTargetPositions _array_element))
        (Default|OpenGrid _array_element)))))

(fn ConstructionScript)
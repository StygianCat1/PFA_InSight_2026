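; BP_Globetrotter is an interactable, possessable puzzle element that the player takes control of.
; Interact relays through multicast and owning-client events to set InteractionActor and have player controller 0 possess it.
; While possessed, IA_Interact hands control back to InteractionActor, while IA_Move and possession only print debug text.
; CanInteract toggles custom depth on ChangeableMesh as a highlight.
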(event Custom|Multicast%20-%20Interact
  (CallFunction|RunonOwningClient-Interact))

(event Custom|RunOnOwningClient%20-%20Interact
  (Variables|Default|SetInteraction%20Actor (stale EventInteract InteractionActor))
  (Pawn|Possess (Game|GetPlayerController 0) self))

(event Input|EnhancedActionEvents|EnhancedInputActionIA_Move
  (params (ActionValue :type Vector%202D%20Structure) (ElapsedSeconds :type Float%20%28double-precision%29) (TriggeredSeconds :type Float%20%28double-precision%29) (InputAction :type Input%20Action%20Object%20Reference :default "/Game/Blueprints/Input/Actions/IA_Move.IA_Move"))
  (:Triggered
    (Development|PrintString "Hello")))

(event Input|EnhancedActionEvents|EnhancedInputActionIA_Interact
  (params (ActionValue :type Boolean) (ElapsedSeconds :type Float%20%28double-precision%29) (TriggeredSeconds :type Float%20%28double-precision%29) (InputAction :type Input%20Action%20Object%20Reference :default "/Game/Blueprints/Input/Actions/IA_Interact.IA_Interact"))
  (:Triggered
    (Pawn|Possess (Game|GetPlayerController 0) (Variables|Default|GetInteraction%20Actor))))

(event EventBeginPlay)

(event Collision|EventActorBeginOverlap
  (params (OtherActor :type Actor%20Object%20Reference)))

(event EventTick
  (params (DeltaSeconds :type Float%20%28single-precision%29)))

(event EventInteract
  (params (InteractionActor :type BP%20First%20Person%20Character%20Object%20Reference))
  (CallFunction|Multicast-Interact))

(event EventPossessed
  (params (NewController :type Controller%20Object%20Reference))
  (Development|PrintString "Hello"))

(fn ConstructionScript)

(fn CanInteract
  (params (CanInteract :type Boolean))
  (Rendering|SetRenderCustomDepth (Variables|Default|GetChangeableMesh) CanInteract)
  (return CanInteract))
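; BP_Pushobject is an interactable puzzle object that Victoria or Walter can grab and move.
; Interacting attaches it to that character, flags them as MovingObject and slows their walk speed; interacting again detaches it and restores the saved speed.
; A MultiGate per character provides the toggle, and grabbing it from the other character releases them and resets their gate.
; CanInteract toggles the cube's custom depth, likely for highlighting.
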(event EventInteract
  (params (InteractionActor :type BP%20First%20Person%20Character%20Object%20Reference))
  (bind _asbp_victoria_character (Utilities|Casting|CastToBP_VictoriaCharacter InteractionActor)
    (:then
      (bind _output_get (Variables|Default|SetVictoriaActor _asbp_victoria_character))
      (Variables|Default|SetVictoriaWalkSpeed (Variables|/Game/Blueprints/CharacterBlueprint/BP_FirstPersonCharacter.BP_FirstPersonCharacter_C|GetWalkSpeed _output_get))
      (Utilities|FlowControl|MultiGate false false -1 :!label _label
        (:Out%200
          (Variables|/Game/Blueprints/CharacterBlueprint/BP_FirstPersonCharacter.BP_FirstPersonCharacter_C|SetMovingObject (Variables|Default|GetVictoriaActor) true)
          (Variables|/Script/Engine.CharacterMovementComponent|SetMaxWalkSpeed (Variables|/Script/Engine.Character|GetCharacterMovement (Variables|Default|GetVictoriaActor)) 1e+02)
          (Variables|Default|GetWalterActor
            (:then
              (Variables|/Game/Blueprints/CharacterBlueprint/BP_FirstPersonCharacter.BP_FirstPersonCharacter_C|SetMovingObject (Variables|Default|GetWalterActor) false)
              (Variables|/Script/Engine.CharacterMovementComponent|SetMaxWalkSpeed (Variables|/Script/Engine.Character|GetCharacterMovement (Variables|Default|GetWalterActor)) (Variables|Default|GetWalterWalkSpeed))
              (Transformation|DetachFromActor "KeepWorld" "KeepWorld" "KeepWorld")
              (Variables|Default|SetWalterActor 0)
              (Utilities|FlowControl|Sequence
                (:then_0
                  _)
                (:then_1
                  (goto _label_2 Reset))))
            (:else
              _))
          (Transformation|AttachActorToActor (Variables|Default|GetVictoriaActor) "None" "KeepWorld" "KeepWorld" "KeepWorld" true))
        (:Out%201
          (Variables|/Game/Blueprints/CharacterBlueprint/BP_FirstPersonCharacter.BP_FirstPersonCharacter_C|SetMovingObject (Variables|Default|GetVictoriaActor) false)
          (Variables|/Script/Engine.CharacterMovementComponent|SetMaxWalkSpeed (Variables|/Script/Engine.Character|GetCharacterMovement (Variables|Default|GetVictoriaActor)) (Variables|Default|GetVictoriaWalkSpeed))
          (Variables|Default|SetVictoriaActor 0)
          (Transformation|DetachFromActor "KeepWorld" "KeepWorld" "KeepWorld")
          (goto _label Reset))))
    (:CastFailed
      (bind _asbp_walter_character (Utilities|Casting|CastToBP_WalterCharacter InteractionActor))
      (bind _output_get_2 (Variables|Default|SetWalterActor _asbp_walter_character))
      (Variables|Default|SetWalterWalkSpeed (Variables|/Game/Blueprints/CharacterBlueprint/BP_FirstPersonCharacter.BP_FirstPersonCharacter_C|GetWalkSpeed _output_get_2))
      (Utilities|FlowControl|MultiGate false false -1 :!label _label_2
        (:Out%200
          (Variables|/Game/Blueprints/CharacterBlueprint/BP_FirstPersonCharacter.BP_FirstPersonCharacter_C|SetMovingObject (Variables|Default|GetWalterActor) true)
          (Variables|/Script/Engine.CharacterMovementComponent|SetMaxWalkSpeed (Variables|/Script/Engine.Character|GetCharacterMovement (Variables|Default|GetWalterActor)) 1e+02)
          (Variables|Default|GetVictoriaActor
            (:then
              (Variables|/Game/Blueprints/CharacterBlueprint/BP_FirstPersonCharacter.BP_FirstPersonCharacter_C|SetMovingObject (Variables|Default|GetVictoriaActor) false)
              (Variables|/Script/Engine.CharacterMovementComponent|SetMaxWalkSpeed (Variables|/Script/Engine.Character|GetCharacterMovement (Variables|Default|GetVictoriaActor)) (Variables|Default|GetVictoriaWalkSpeed))
              (Transformation|DetachFromActor "KeepWorld" "KeepWorld" "KeepWorld")
              (Variables|Default|SetVictoriaActor 0)
              (Utilities|FlowControl|Sequence
                (:then_0
                  _)
                (:then_1
                  (goto _label Reset))))
            (:else
              _))
          (Transformation|AttachActorToActor (Variables|Default|GetWalterActor) "None" "KeepWorld" "KeepWorld" "KeepWorld" true))
        (:Out%201
          (Variables|/Game/Blueprints/CharacterBlueprint/BP_FirstPersonCharacter.BP_FirstPersonCharacter_C|SetMovingObject (Variables|Default|GetWalterActor) false)
          (Variables|/Script/Engine.CharacterMovementComponent|SetMaxWalkSpeed (Variables|/Script/Engine.Character|GetCharacterMovement (Variables|Default|GetWalterActor)) (Variables|Default|GetWalterWalkSpeed))
          (Variables|Default|SetWalterActor 0)
          (Transformation|DetachFromActor "KeepWorld" "KeepWorld" "KeepWorld")
          (goto _label_2 Reset))))))

(event EventBeginPlay)

(fn ConstructionScript)

(fn CanInteract
  (params (CanInteract :type Boolean))
  (Rendering|SetRenderCustomDepth (Variables|Default|GetCube) CanInteract)
  (return CanInteract))
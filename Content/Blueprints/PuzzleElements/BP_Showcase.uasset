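; BP_Showcase is a puzzle-element showcase whose top swings open once when its Interact event fires.
; BeginPlay caches the top's starting pitch, then Interact passes a DoOnce, plays a sound and runs the OpenShowcase timeline to add up to OpenAngle to that pitch.
; CanInteract always returns false, and the file contains no reset or closing logic.
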(event EventBeginPlay
  (Variables|Default|SetInitialRotation (.pitch (Variables|/Script/Engine.SceneComponent|GetRelativeRotation (Variables|Default|GetShowcaseTop)))))

(event EventInteract
  (params (InteractionActor :type BP%20First%20Person%20Character%20Object%20Reference))
  (Utilities|FlowControl|DoOnce false
    (:Completed
      (Audio|PlaySoundatLocation "/Game/Sound/SFX/Base/Importer/Showcase.Showcase" (Transformation|GetActorLocation) "0, 0, 0" 1.0 1.0 0.0 0 0 0 0)
      (bind _open (Timeline|OpenShowcase PlayFromStart)
        (:Update
          (Transformation|SetRelativeRotation (Variables|Default|GetShowcaseTop) (Math|Rotator|MakeRotator 0.0 (+ (Variables|Default|GetInitialRotation) (* _open (Variables|Default|GetOpenAngle))) 0.0) false false))))))

(fn ConstructionScript)

(fn CanInteract
  (params (CanInteract :type Boolean))
  (return false))
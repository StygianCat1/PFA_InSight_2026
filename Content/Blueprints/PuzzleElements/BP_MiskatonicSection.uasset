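; BP_MiskatonicSection is a puzzle element that opens a secret passage once and then advances the eldritch circle.
; OpenPassage plays an unlock sound, waits, then plays a door sound while a timeline yaws RotationPoint.
; When the swing finishes, it calls ActivateCandle after a short delay on the BP_EldritchCirrcle found at BeginPlay.
; CanInteract always returns false, and an older bookcase-sliding timeline remains unconnected.
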(event Custom|OpenPassage
  (bind _rotation_point (Variables|Default|GetRotation%20Point))
  (bind _relativelocation (Variables|/Script/Engine.SceneComponent|GetRelativeLocation _rotation_point))
  (Utilities|FlowControl|DoOnce false
    (:Completed
      (Variables|Default|SetRelative%20Location _relativelocation)
      (Audio|PlaySoundatLocation "/Game/Sound/SFX/Base/Importer/UnlockSecretDoor.UnlockSecretDoor" _relativelocation "0, 0, 0" 1.0 1.0 0.0 0 0 0 0)
      (Utilities|FlowControl|Delay 3.5)
      (Audio|PlaySoundatLocation "/Game/Sound/SFX/Base/Importer/OpenWood_door.OpenWood_door" _relativelocation "0, 0, 0" 1.0 1.0 0.0 0 0 0 0)
      (bind _z_rotation (Timeline|Timeline_0 PlayFromStart)
        (:Update
          (Transformation|SetRelativeRotation (Variables|Default|GetRotation%20Point) (Math|Rotator|MakeRotator 0.0 0.0 _z_rotation) false false))
        (:Finished
          (Utilities|FlowControl|Delay 1.0)
          (bind _eldritchcircle (Variables|Default|GetEldritchCircle)
            (:then
              (Default|ActivateCandle _eldritchcircle))
            (:else)))))))

(event EventBeginPlay
  (bind _returnvalue (Actor|GetActorOfClass "/Game/Blueprints/PuzzleElements/BP_EldritchCirrcle.BP_EldritchCirrcle_C"))
  (Variables|Default|SetEldritchCircle _returnvalue))

(fn ConstructionScript)

(fn CanInteract
  (params (CanInteract :type Boolean))
  (return false))
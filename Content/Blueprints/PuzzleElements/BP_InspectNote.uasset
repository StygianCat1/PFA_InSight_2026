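; BP_InspectNote is an interactable note puzzle element whose item mesh hides and reappears on alternate interactions.
; On BeginPlay it applies the ItemMesh variable to its Item component.
; Interact uses a FlipFlop to toggle the Item's visibility, starting with hiding it.
; CanInteract passes its input flag to the Item's custom depth rendering, likely for highlighting, and returns the same value.
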(event EventBeginPlay
  (Components|StaticMesh|SetStaticMesh (Variables|Default|GetItem) (Variables|Default|GetItemMesh)))

(event EventInteract
  (params (InteractionActor :type BP%20First%20Person%20Character%20Object%20Reference))
  (bind _item (Variables|Default|GetItem))
  (Utilities|FlowControl|FlipFlop
    (:A
      (Rendering|SetVisibility _item false false))
    (:B
      (Rendering|SetVisibility _item true false))))

(fn ConstructionScript)

(fn CanInteract
  (params (CanInteract :type Boolean))
  (Rendering|SetRenderCustomDepth (Variables|Default|GetItem) CanInteract)
  (return CanInteract))
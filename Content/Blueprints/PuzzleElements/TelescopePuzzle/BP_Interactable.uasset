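; Collectible for the telescope puzzle that grants astronomy parts and shows a discovery popup when interacted with.
; On BeginPlay it totals Number across all instances sharing its ObjectName and caches the BP_MapImage actor.
; A one-time Interact adds Number to the interactor's AstronomyPart, optionally updates the map, displays count and description, then destroys the actor.
; CanInteract toggles custom depth on the mesh for highlighting.
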(event EventInteract
  (params (InteractionActor :type BP%20First%20Person%20Character%20Object%20Reference))
  (Utilities|FlowControl|DoOnce false
    (:Completed
      (bind _output_get (Variables|Default|SetInteraction%20Actor InteractionActor))
      (bind _output_get_2 (Variables|/Game/Blueprints/CharacterBlueprint/BP_FirstPersonCharacter.BP_FirstPersonCharacter_C|SetAstronomyPart _output_get (+ (Variables|Default|GetNumber) (Variables|/Game/Blueprints/CharacterBlueprint/BP_FirstPersonCharacter.BP_FirstPersonCharacter_C|GetAstronomyPart _output_get))))
      (if (Variables|Default|GetChangeMap)
        (bind _mapparttotal (Variables|Default|GetMapPartTotal)
          (:then
            (Default|CallChangeValue _mapparttotal))
          (:else
            _)))
      (if (> (Variables|Default|GetTotal%20Number) 1)
        (Variables|Default|SetNumberText (Utilities|String|Append (Utilities|String|ToString(Integer) _output_get_2) "/" (Utilities|String|ToString(Integer) (Variables|Default|GetTotal%20Number))))
        (else
          (Variables|Default|SetNumberText (Utilities|String|ToString(Integer) _output_get_2))))
      (bind _returnvalue (UserInterface|CreateWidget "/Game/UI/Others/WBP_InformationOnDiscovery.WBP_InformationOnDiscovery_C" 0 (Variables|Default|GetNumberText) (Variables|Default|GetObjectName) (Variables|Default|GetDescription)))
      (UserInterface|Viewport|AddtoViewport _returnvalue 0)
      (Utilities|FlowControl|Delay 0.025)
      (Actor|DestroyActor))))

(event EventBeginPlay
  (bind _returnvalue (Actor|GetActorOfClass "/Game/Blueprints/PuzzleElements/TelescopePuzzle/BP_MapImage.BP_MapImage_C"))
  (Variables|Default|SetMapPartTotal _returnvalue)
  (bind _outactors (Actor|GetAllActorsOfClass "BP_Interactable_C"))
  (for _array_element _outactors
    (if (== (Variables|BP_Interactable_C|GetObjectName _array_element) (Variables|Default|GetObjectName))
      (Utilities|Array|AddUnique (Variables|Default|GetRefToActorOfSameName) _array_element)
      (Variables|Default|SetTotal%20Number (+ (Variables|Default|GetTotal%20Number) (Variables|Default|GetNumber))))))

(fn ConstructionScript)

(fn CanInteract
  (params (CanInteract :type Boolean))
  (Rendering|SetRenderCustomDepth (Variables|Default|GetStaticMesh) CanInteract)
  (return CanInteract))
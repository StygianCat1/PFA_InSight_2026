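; BP_Telescope is an interactable telescope puzzle element that shows a view widget to the locally viewed interacting player.
; On BeginPlay it finds the BP_ChangeImage and BP_ImageClarity actors, whose current image and clarity seed WBP_TelescopeView on opening.
; A resetting MultiGate toggles Interact between showing the widget with move and look input locked, and removing it to restore input.
; CanInteract also toggles the mesh's custom depth rendering.
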(event EventInteract
  (params (InteractionActor :type BP%20First%20Person%20Character%20Object%20Reference))
  (bind _output_get (Variables|Default|SetInteraction%20Actor InteractionActor))
  (if (Pawn|IsLocallyViewed _output_get)
    (Utilities|FlowControl|MultiGate false false -1 :!label _label
      (:Out%200
        (Input|SetIgnoreMoveInput (Pawn|GetLocalViewingPlayerController (Variables|Default|GetInteraction%20Actor)) true)
        (Input|SetIgnoreLookInput (Pawn|GetLocalViewingPlayerController (Variables|Default|GetInteraction%20Actor)) true)
        (bind _returnvalue (UserInterface|CreateWidget "/Game/UI/Other/WBP_TelescopeView.WBP_TelescopeView_C" 0 (Variables|/Game/Blueprints/PuzzleElements/TelescopePuzzle/BP_ImageClarity.BP_ImageClarity_C|GetClarity (Variables|Default|GetImageClarityBlueprintRef)) (Variables|/Game/Blueprints/PuzzleElements/TelescopePuzzle/BP_ChangeImage.BP_ChangeImage_C|GetImage (Variables|Default|GetChangeImageBlueprintref))))
        (bind _output_get_2 (Variables|Default|SetWidgetRef _returnvalue))
        (UserInterface|Viewport|AddtoViewport _returnvalue 0))
      (:Out%201
        (Widget|RemovefromParent (Variables|Default|GetWidgetRef))
        (Input|ResetIgnoreMoveInput (Pawn|GetLocalViewingPlayerController (Variables|Default|GetInteraction%20Actor)))
        (Input|ResetIgnoreLookInput (Pawn|GetLocalViewingPlayerController (Variables|Default|GetInteraction%20Actor)))
        (goto _label Reset)))))

(event EventBeginPlay
  (bind _returnvalue (Actor|GetActorOfClass "/Game/Blueprints/PuzzleElements/TelescopePuzzle/BP_ChangeImage.BP_ChangeImage_C"))
  (Variables|Default|SetChangeImageBlueprintref _returnvalue)
  (bind _returnvalue_2 (Actor|GetActorOfClass "/Game/Blueprints/PuzzleElements/TelescopePuzzle/BP_ImageClarity.BP_ImageClarity_C"))
  (Variables|Default|SetImageClarityBlueprintRef _returnvalue_2))

(fn ConstructionScript)

(fn CanInteract
  (params (CanInteract :type Boolean))
  (Rendering|SetRenderCustomDepth (Variables|Default|GetStaticMesh) CanInteract)
  (return CanInteract))
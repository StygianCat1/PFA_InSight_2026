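; Interactable telescope puzzle element that rotates its mesh to step through three images.
; Interact plays a timeline that turns the mesh's yaw up to 120 degrees from the stored position.
; When it finishes, it saves the new yaw, cycles the image index from 1 to 3, and resets the timeline.
; CanInteract toggles custom depth on the mesh, passing the interactable state through.
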(event EventBeginPlay)

(event Collision|EventActorBeginOverlap
  (params (OtherActor :type Actor%20Object%20Reference)))

(event EventTick
  (params (DeltaSeconds :type Float%20%28single-precision%29)))

(event EventInteract
  (params (InteractionActor :type BP%20First%20Person%20Character%20Object%20Reference))
  (bind _staticmesh (Variables|Default|GetStaticMesh))
  (bind _relativerotation (Variables|/Script/Engine.SceneComponent|GetRelativeRotation _staticmesh))
  (bind _turnlenght (Timeline|Timeline Play)
    (:Update
      (Transformation|SetRelativeRotation _staticmesh (Math|Rotator|MakeRotator (.roll _relativerotation) (.pitch _relativerotation) (+ (Variables|Default|GetRelativePosition) (* _turnlenght 1.2e+02))) false false))
    (:Finished
      (Variables|Default|SetRelativePosition (.yaw (Variables|/Script/Engine.SceneComponent|GetRelativeRotation (Variables|Default|GetStaticMesh))))
      (if (> (+ (Variables|Default|GetImage) 1) 3)
        (Variables|Default|SetImage 1)
        (Timeline|Timeline SetNewTime)
        (else
          (Variables|Default|SetImage (+ (Variables|Default|GetImage) 1))
          (Timeline|Timeline SetNewTime))))))

(fn ConstructionScript)

(fn CanInteract
  (params (CanInteract :type Boolean))
  (Rendering|SetRenderCustomDepth (Variables|Default|GetStaticMesh) CanInteract)
  (return CanInteract))
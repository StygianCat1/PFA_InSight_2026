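; Interactable image clarity control for the telescope puzzle, a mesh that rotates through three positions.
; Each interaction plays a timeline that rolls the mesh a further 120 degrees, then stores the new roll and resets the timeline.
; When the turn finishes, Clarity advances, wrapping from 3 back to 1.
; CanInteract toggles the mesh's custom depth rendering to match interactability.
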(event EventInteract
  (params (InteractionActor :type BP%20First%20Person%20Character%20Object%20Reference))
  (bind _staticmesh (Variables|Default|GetStaticMesh))
  (bind _relativerotation (Variables|/Script/Engine.SceneComponent|GetRelativeRotation _staticmesh))
  (bind _turnlenght (Timeline|TurnObject Play)
    (:Update
      (Transformation|SetRelativeRotation _staticmesh (Math|Rotator|MakeRotator (+ (Variables|Default|GetRelativePosition) (* _turnlenght 1.2e+02)) (.pitch _relativerotation) (.yaw _relativerotation)) false false))
    (:Finished
      (Variables|Default|SetRelativePosition (.roll (Variables|/Script/Engine.SceneComponent|GetRelativeRotation (Variables|Default|GetStaticMesh))))
      (if (> (+ (Variables|Default|GetClarity) 1) 3)
        (Variables|Default|SetClarity 1)
        (Timeline|TurnObject SetNewTime)
        (else
          (Variables|Default|SetClarity (+ (Variables|Default|GetClarity) 1))
          (Timeline|TurnObject SetNewTime))))))

(fn ConstructionScript)

(fn CanInteract
  (params (CanInteract :type Boolean))
  (Rendering|SetRenderCustomDepth (Variables|Default|GetStaticMesh) CanInteract)
  (return CanInteract))
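; Interactable puzzle door that swings open to the left or right on Interact and closes on the next use.
; A MultiGate alternates between playing and reversing the Move timeline, resetting only once the closing finishes.
; The timeline scales the chosen side's yaw on the Scene pivot, while roll and pitch apply unscaled.
; CanInteract toggles custom depth on the Cube and always returns false.
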(event EventInteract
  (bind _openrightrot (Variables|Default|GetOpenRightRot))
  (bind _openleftrot (Variables|Default|GetOpenLeftRot))
  (Utilities|FlowControl|MultiGate false false -1 :!label _label
    (:Out%200
      (bind (_direction _doortrack) (Timeline|Move Play)
        (:Update
          (switch Utilities|FlowControl|Switch|SwitchonE_DoorSide (Variables|Default|GetDoorOpeningSide)
            (:NewEnumerator0
              (Transformation|SetRelativeRotation (Variables|Default|GetScene) (Math|Rotator|MakeRotator (.roll _openrightrot) (.pitch _openrightrot) (* _doortrack (.yaw _openrightrot))) false false))
            (:NewEnumerator1
              (Transformation|SetRelativeRotation (Variables|Default|GetScene) (Math|Rotator|MakeRotator (.roll _openleftrot) (.pitch _openleftrot) (* _doortrack (.yaw _openleftrot))) false false))))
        (:Finished
          (switch Utilities|FlowControl|Switch|SwitchonETimelineDirection _direction
            (:Backward
              (goto _label Reset))))))
    (:Out%201
      (Timeline|Move Reverse))))

(fn ConstructionScript)

(fn CanInteract
  (params (CanInteract :type Boolean))
  (Rendering|SetRenderCustomDepth (Variables|Default|GetCube) CanInteract)
  (return false))
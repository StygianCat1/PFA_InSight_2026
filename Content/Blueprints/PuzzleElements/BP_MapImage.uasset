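; BP_MapImage is a puzzle-element map image that reveals itself in three parts as progress events arrive.
; On BeginPlay it binds IncrementMapPartNumber through BindEventToChangeValue.
; Each call increments NumberOfCall and switches on it to make Part1, Part2 or Part3 visible.
; NumberOfCall has a RepNotify function, but that function is empty.
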(event Custom|IncrementMapPartNumber
  (bind _result (Math|Integer|IncrementInt (Variables|Default|GetNumberOfCall))
    (:%20%20
      (switch int _result
        (:1
          (Rendering|SetVisibility (Variables|Default|GetPart1) true false))
        (:2
          (Rendering|SetVisibility (Variables|Default|GetPart2) true false))
        (:3
          (Rendering|SetVisibility (Variables|Default|GetPart3) true false))))))

(event EventBeginPlay
  (EventDispatchers|BindEventtoChangeValue (delegate Custom|IncrementMapPartNumber)))

(fn ConstructionScript)

(fn OnRepNumberOfCall)
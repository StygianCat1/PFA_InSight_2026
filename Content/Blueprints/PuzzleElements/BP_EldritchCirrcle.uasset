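; Eldritch circle puzzle element that lights candles and opens a descending staircase.
; Each ActivateCandle call increments a counter and uses a MultiGate to light the next of four pillars.
; Interact runs a one-time incantation, hides the circle and its collision, then lowers stairs to stepped depths via MoveComponentTo.
; CanInteract returns false, and the candle-count check leading to that sequence is disconnected.
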(event Custom|DeployStairs
  (bind _stair_06 (Variables|Default|GetStair_06))
  (bind _stair_07 (Variables|Default|GetStair_07))
  (bind _stair_08 (Variables|Default|GetStair_08))
  (bind _stair_09 (Variables|Default|GetStair_09))
  (bind _stair_10 (Variables|Default|GetStair_10))
  (bind _stair_11 (Variables|Default|GetStair_11))
  (bind _stair_12 (Variables|Default|GetStair_12))
  (bind _stair_02 (Variables|Default|GetStair_02))
  (bind _stair_03 (Variables|Default|GetStair_03))
  (bind _stair_04 (Variables|Default|GetStair_04))
  (bind _stair_05 (Variables|Default|GetStair_05))
  (Components|MoveComponentTo _stair_02 (- (Variables|/Script/Engine.SceneComponent|GetRelativeLocation _stair_02) "0.000000,0.000000,30.000000") (Variables|/Script/Engine.SceneComponent|GetRelativeRotation _stair_02) false false 0.2 false)
  (Components|MoveComponentTo _stair_03 (- (Variables|/Script/Engine.SceneComponent|GetRelativeLocation _stair_03) "0.000000,0.000000,60.000000") (Variables|/Script/Engine.SceneComponent|GetRelativeRotation _stair_03) false false 0.2 false)
  (Components|MoveComponentTo _stair_04 (- (Variables|/Script/Engine.SceneComponent|GetRelativeLocation _stair_04) "0.000000,0.000000,90.000000") (Variables|/Script/Engine.SceneComponent|GetRelativeRotation _stair_04) false false 0.2 false)
  (Components|MoveComponentTo _stair_05 (- (Variables|/Script/Engine.SceneComponent|GetRelativeLocation _stair_05) "0.000000,0.000000,120.000000") (Variables|/Script/Engine.SceneComponent|GetRelativeRotation _stair_05) false false 0.2 false)
  (Components|MoveComponentTo _stair_06 (- (Variables|/Script/Engine.SceneComponent|GetRelativeLocation _stair_06) "0.000000,0.000000,150.000000") (Variables|/Script/Engine.SceneComponent|GetRelativeRotation _stair_06) false false 0.2 false)
  (Components|MoveComponentTo _stair_07 (- (Variables|/Script/Engine.SceneComponent|GetRelativeLocation _stair_07) "0.000000,0.000000,180.000000") (Variables|/Script/Engine.SceneComponent|GetRelativeRotation _stair_07) false false 0.2 false)
  (Components|MoveComponentTo _stair_08 (- (Variables|/Script/Engine.SceneComponent|GetRelativeLocation _stair_08) "0.000000,0.000000,210.000000") (Variables|/Script/Engine.SceneComponent|GetRelativeRotation _stair_08) false false 0.2 false)
  (Components|MoveComponentTo _stair_09 (- (Variables|/Script/Engine.SceneComponent|GetRelativeLocation _stair_09) "0.000000,0.000000,240.000000") (Variables|/Script/Engine.SceneComponent|GetRelativeRotation _stair_09) false false 0.2 false)
  (Components|MoveComponentTo _stair_10 (- (Variables|/Script/Engine.SceneComponent|GetRelativeLocation _stair_10) "0.000000,0.000000,270.000000") (Variables|/Script/Engine.SceneComponent|GetRelativeRotation _stair_10) false false 0.2 false)
  (Components|MoveComponentTo _stair_11 (- (Variables|/Script/Engine.SceneComponent|GetRelativeLocation _stair_11) "0.000000,0.000000,300.000000") (Variables|/Script/Engine.SceneComponent|GetRelativeRotation _stair_11) false false 0.2 false)
  (Components|MoveComponentTo _stair_12 (- (Variables|/Script/Engine.SceneComponent|GetRelativeLocation _stair_12) "0.000000,0.000000,330.000000") (Variables|/Script/Engine.SceneComponent|GetRelativeRotation _stair_12) false false 0.2 false))

(event Custom|ActivateCandle
  (Math|Integer|IncrementInt (Variables|Default|GetCandleCounter)
    (:%20%20
      (Audio|PlaySoundatLocation "/Game/Sound/SFX/Cue/Allumage_Bougie_WitheFade_Cue.Allumage_Bougie_WitheFade_Cue" (Transformation|GetActorLocation) "0, 0, 0" 1.0 1.0 0.0 0 0 0 0)
      (Utilities|FlowControl|MultiGate false false -1
        (:Out%200
          (Rendering|Material|SetMaterial (Variables|Default|GetPillar1) 0 "/Game/Materials/BasicUnrealMaterial/MI_Blue.MI_Blue")
          (Components|Activation|Activate (Variables|Default|GetCandle1) false))
        (:Out%201
          (Rendering|Material|SetMaterial (Variables|Default|GetPillar2) 0 "/Game/Materials/BasicUnrealMaterial/MI_Blue.MI_Blue")
          (Components|Activation|Activate (Variables|Default|GetCandle2) false))
        (:Out%202
          (Rendering|Material|SetMaterial (Variables|Default|GetPillar3) 0 "/Game/Materials/BasicUnrealMaterial/MI_Blue.MI_Blue")
          (Components|Activation|Activate (Variables|Default|GetCandle3) false))
        (:Out%203
          (Rendering|Material|SetMaterial (Variables|Default|GetPillar4) 0 "/Game/Materials/BasicUnrealMaterial/MI_Blue.MI_Blue")
          (Components|Activation|Activate (Variables|Default|GetCandle4) false))))))

(event Custom|VanishBase
  (bind _circle (Variables|Default|GetCircle))
  (Rendering|Material|SetMaterial _circle 0 "/Game/Materials/BasicUnrealMaterial/M_Transparent.M_Transparent")
  (Collision|SetCollisionEnabled _circle "NoCollision"))

(event EventInteract
  (params (InteractionActor :type BP%20First%20Person%20Character%20Object%20Reference))
  (Utilities|FlowControl|DoOnce false
    (:Completed
      (Components|Activation|Activate (Variables|Default|GetIncantation) true)
      (Utilities|FlowControl|Delay 7.0)
      (Components|Activation|Deactivate (Variables|Default|GetIncantation))
      (CallFunction|VanishBase)
      (Utilities|FlowControl|Delay 1.0)
      (CallFunction|DeployStairs))))

(fn ConstructionScript)

(fn CanInteract
  (params (CanInteract :type Boolean))
  (return false))
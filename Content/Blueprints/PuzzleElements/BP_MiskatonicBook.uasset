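; Interactable puzzle book, spawned as a child actor of BP_MiskatonicSection, that tilts to help open a hidden passage.
; Interact alternately plays and reverses a tilt timeline, whose finish updates this book's entry, indexed by BookNumber, in the parent's BookStates.
; When that array matches TargetBookStates, it calls OpenPassage on the parent.
; CanInteract toggles custom depth on the mesh; older toggle variants remain unconnected.
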(event EventBeginPlay
  (Variables|Default|SetBookRotation (.pitch (Transformation|GetWorldRotation (Variables|Default|GetMiskatonicBook))))
  (bind _asbp_miskatonic_section (Utilities|Casting|CastToBP_MiskatonicSection (Actor|GetParentActor self)))
  (Variables|Default|SetBookcase _asbp_miskatonic_section))

(event EventInteract
  (bind _bookcase (Variables|Default|GetBookcase))
  (bind _booknumber (Variables|Default|GetBookNumber))
  (bind _returnvalue (- _booknumber 1))
  (bind _bookstates (Variables|/Game/Blueprints/PuzzleElements/BP_MiskatonicSection.BP_MiskatonicSection_C|GetBookStates _bookcase))
  (bind _output (Utilities|Array|Get(acopy) _bookstates _returnvalue))
  (bind _returnvalue_2 (not _output))
  (Development|PrintString "Hello")
  (Utilities|FlowControl|FlipFlop
    (:A
      (bind _tilt (Timeline|Timeline_0 Play)
        (:Update
          (Transformation|SetWorldRotation (Variables|Default|GetMiskatonicBook) (Math|Rotator|MakeRotator 0.0 (+ (Variables|Default|GetBookRotation) (* _tilt (Variables|Default|GetTiltAngle))) 0.0) false false))
        (:Finished
          (Variables|Default|SetBookRotation 0.0)
          (Development|PrintString (Utilities|String|Append "Index: " (Utilities|String|ToString(Integer) _booknumber) " & State: " (Utilities|String|ToString(Boolean) _returnvalue_2)))
          (if _returnvalue_2
            (Utilities|Array|SetArrayElem _bookstates _returnvalue _returnvalue_2)
            (Development|PrintString "Desact")
            (else
              (Utilities|Array|SetArrayElem _bookstates _returnvalue false)
              (Development|PrintString "Act")))
          (if (Utilities|Array|Identical _bookstates (Variables|/Game/Blueprints/PuzzleElements/BP_MiskatonicSection.BP_MiskatonicSection_C|GetTargetBookStates _bookcase))
            (Default|OpenPassage _bookcase)))))
    (:B
      (Timeline|Timeline_0 Reverse))))

(fn ConstructionScript)

(fn CanInteract
  (params (CanInteract :type Boolean))
  (Rendering|SetRenderCustomDepth (Variables|Default|GetMiskatonicBook) CanInteract)
  (return false))
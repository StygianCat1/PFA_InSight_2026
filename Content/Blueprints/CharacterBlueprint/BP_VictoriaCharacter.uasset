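; Victoria's playable character Blueprint, which learns its gameplay abilities on BeginPlay and handles starting and stopping two of them through the Gameplay Ability System.
; Use and stop functions call Multicast events that forward to RunOnServer events.
; Start events activate abilities by class.
; Stop events fetch the ability from its stored spec handle and send it a stop message, with ability 2 also calling Cooldown.
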(event Custom|RunOnServer%20-%20VictoriaStopUseAbility2
  (Class|BPICapacity|StopCapacity2(Message) (.ReturnValue (Ability|GameplayAbility|GetGameplayAbilityfromSpecHandle (Variables|Default|GetAbilitySystem) (Variables|Default|GetCapacity2SpecHandle))) self (Variables|Default|GetCheckCapacity2))
  (CallFunction|Cooldown))

(event Custom|Multicast%20-%20VictoriaStopUseAbility2
  (CallFunction|RunonServer-VictoriaStopUseAbility2))

(event Custom|RunOnServer%20-%20VictoriaStopUseAbility1
  (Class|BPICapacity|StopCapacity1(Message) (.ReturnValue (Ability|GameplayAbility|GetGameplayAbilityfromSpecHandle (Variables|Default|GetAbilitySystem) (Variables|Default|GetCapacity1SpecHandle))) self (Variables|Default|GetCheckCapacity1)))

(event Custom|Multicast%20-%20VictoriaUseAbility2
  (CallFunction|RunonServer-VictoriaUseAbility2))

(event Custom|RunOnServer%20-%20VictoriaUseAbility2
  (Abilities|TryActivateAbilitybyClass (Variables|Default|GetAbilitySystem) (Variables|Default|GetGameplayAbilty2) true))

(event Custom|Multicast%20-%20VictoriaUseAbility1
  (CallFunction|RunonServer-VictoriaUseAbility1))

(event Custom|RunOnServer%20-%20VictoriaUseAbility1
  (Abilities|TryActivateAbilitybyClass (Variables|Default|GetAbilitySystem) (Variables|Default|GetGameplayAbilty1) true))

(event Custom|Multicast%20-%20VictoriaStopUseAbility1
  (CallFunction|RunonServer-VictoriaStopUseAbility1))

(event EventBeginPlay
  (|CallParentFunction)
  (CallFunction|LearnGameplayAbility))

(fn ConstructionScript
  (|CallParentFunction))

(fn UseAbility1
  (CallFunction|Multicast-VictoriaUseAbility1))

(fn UseAbility2
  (CallFunction|Multicast-VictoriaUseAbility2))

(fn StopUseAbility1
  (CallFunction|Multicast-VictoriaStopUseAbility1))

(fn StopUseAbility2
  (CallFunction|Multicast-VictoriaStopUseAbility2))

(fn RunonServer-UseAbility1)
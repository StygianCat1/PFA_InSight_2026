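; Walter character Blueprint that learns its gameplay abilities on BeginPlay and handles starting and stopping two of them.
; Use and stop functions call Multicast-named events, which forward to RunOnServer-named events.
; Those events activate each ability by class through the Ability System, or fetch it by spec handle and send it a stop message.
; Stopping the second ability also calls Cooldown.
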(event Custom|RunOnServer%20-%20WalterStopUseAbility2
  (Class|BPICapacity|StopCapacity2(Message) (.ReturnValue (Ability|GameplayAbility|GetGameplayAbilityfromSpecHandle (Variables|Default|GetAbilitySystem) (Variables|Default|GetCapacity2SpecHandle))) self (Variables|Default|GetCheckCapacity2))
  (CallFunction|Cooldown))

(event Custom|Multicast%20-%20WalterStopUseAbility2
  (CallFunction|RunonServer-WalterStopUseAbility2))

(event Custom|RunOnServer%20-%20WalterStopUseAbility1
  (Class|BPICapacity|StopCapacity1(Message) (.ReturnValue (Ability|GameplayAbility|GetGameplayAbilityfromSpecHandle (Variables|Default|GetAbilitySystem) (Variables|Default|GetCapacity1SpecHandle))) self (Variables|Default|GetCheckCapacity1)))

(event Custom|Multicast%20-%20WalterUseAbility2
  (CallFunction|RunonServer-WalterUseAbility2))

(event Custom|RunOnServer%20-%20WalterUseAbility2
  (Abilities|TryActivateAbilitybyClass (Variables|Default|GetAbilitySystem) (Variables|Default|GetGameplayAbilty2) true))

(event Custom|Multicast%20-%20WalterUseAbility1
  (CallFunction|RunonServer-WalterUseAbility1))

(event Custom|RunOnServer%20-%20WalterUseAbility1
  (Abilities|TryActivateAbilitybyClass (Variables|Default|GetAbilitySystem) (Variables|Default|GetGameplayAbilty1) true))

(event Custom|Multicast%20-%20WalterStopUseAbility1
  (CallFunction|RunonServer-WalterStopUseAbility1))

(event EventBeginPlay
  (|CallParentFunction)
  (CallFunction|LearnGameplayAbility))

(fn ConstructionScript
  (|CallParentFunction))

(fn UseAbility1
  (CallFunction|Multicast-WalterUseAbility1))

(fn UseAbility2
  (CallFunction|Multicast-WalterUseAbility2))

(fn StopUseAbility1
  (CallFunction|Multicast-WalterStopUseAbility1))

(fn StopUseAbility2
  (CallFunction|Multicast-WalterStopUseAbility2))